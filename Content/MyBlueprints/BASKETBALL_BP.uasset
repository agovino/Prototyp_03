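; Basketball actor that a VR motion controller can pick up and drop.
; Pickup turns off mesh physics and attaches the root to the given component, while Drop restores physics and detaches, both keeping world transform.
; A BallScale event maps an alpha to a uniform actor scale between half and full size.
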(event Custom|BallScale
  (params (BallScale :type Float%20%28single-precision%29))
  (bind _returnvalue (Math|Float|Lerp 0.5 1.0 BallScale))
  (Transformation|SetActorScale3D (Math|Vector|MakeVector _returnvalue _returnvalue _returnvalue)))

(event EventPickup
  (params (AttachTo :type Scene%20Component%20Object%20Reference))
  (Physics|SetSimulatePhysics (Variables|Debug|GetStaticMeshComponent) false)
  (Transformation|AttachComponentToComponent (VehicleSound|GetRootComponent) AttachTo "None" "KeepWorld" "KeepWorld" "KeepWorld" false))

(event EventDrop
  (Physics|SetSimulatePhysics (Variables|Debug|GetStaticMeshComponent) true)
  (Transformation|DetachFromActor "KeepWorld" "KeepWorld" "KeepWorld"))

(fn ConstructionScript)